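; BP_NPC_AI is an AI controller for guard NPCs that runs the GuardBehaviour tree on the PatrolData blackboard.
; Perception updates from actors without the "Guard" tag toggle IsAiming on the controlled BP_Character according to whether the stimulus was sensed.
; A successful sense writes player 0's pawn, rather than the sensed actor, to a blackboard key, and a lost stimulus clears it.
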(event `self.ReceiveBeginPlay`
  ;[1 1 1] Set Blackboard Component
  (bind _blackboardcomponent (`self.UseBlackboard` "/Game/Dynamic/Character/AI/PatrolData.PatrolData"))
  (set `self.BlackboardComp` _blackboardcomponent)
  (`self.RunBehaviorTree` "/Game/Dynamic/Character/AI/GuardBehaviour.GuardBehaviour"))

(event `self.AIPerception.OnTargetPerceptionUpdated`
  (params (Actor :type "Actor Object Reference") (Stimulus :type "AIStimulus Structure"))
  (bind (_age _expirationage _strength _stimuluslocation _receiverlocation _tag _bsuccessfullysensed) (break `AIStimulus` Stimulus))
  (`AIPerceptionSystem.GetSenseClassForStimulus` Stimulus)
  (if (not (`self.ActorHasTag` Actor "Guard"))
    (`self.SetAiming` _bsuccessfullysensed)
    (if _bsuccessfullysensed
      (`BlackboardComponent.SetValueAsObject` (`self.BlackboardComp`) (`self.KeyName`) (`self.K2_GetPawn` (`GameplayStatics.GetPlayerController` 0)))
      (else
        (`BlackboardComponent.ClearValue` (`self.BlackboardComp`) (`self.KeyName`))))))

(fn `SetAiming`
  (params (IsAiming :type Boolean))
  (bind _asbp_character (cast `/Game/Dynamic/Character/Behaviour/BP_Character` (`self.K2_GetPawn`)))
  (set `/Game/Dynamic/Character/Behaviour/BP_Character.IsAiming` IsAiming _asbp_character))

(fn `UserConstructionScript`)