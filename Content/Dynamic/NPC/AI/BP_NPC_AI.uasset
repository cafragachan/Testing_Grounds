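; BP_NPC_AI is the AI logic for guard NPCs, starting the GuardBehaviour tree on the PatrolData blackboard at BeginPlay.
; AI perception updates ignore actors tagged "Guard" and drive a single blackboard key.
; A successful sense stores player 0's pawn in that key, whichever actor was sensed, and a failed sense clears it.
; The stimulus's sense class is looked up but never used.
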(event `self.ReceiveBeginPlay`
  ;[1 1 1] Set Blackboard Component
  (bind _blackboardcomponent (`self.UseBlackboard` "/Game/Dynamic/NPC/AI/PatrolData.PatrolData"))
  (set `self.BlackboardComp` _blackboardcomponent)
  (`self.RunBehaviorTree` "/Game/Dynamic/NPC/AI/GuardBehaviour.GuardBehaviour"))

(event `self.AIPerception.OnTargetPerceptionUpdated`
  (params (Actor :type "Actor Object Reference") (Stimulus :type "AIStimulus Structure"))
  (`AIPerceptionSystem.GetSenseClassForStimulus` Stimulus)
  (if (`self.ActorHasTag` Actor "Guard")
    _
    (elif (`.bSuccessfullySensed` (break `AIStimulus` Stimulus))
      (`BlackboardComponent.SetValueAsObject` (`self.BlackboardComp`) (`self.KeyName`) (`self.K2_GetPawn` (`GameplayStatics.GetPlayerController` 0)))
      (else
        (`BlackboardComponent.ClearValue` (`self.BlackboardComp`) (`self.KeyName`))))))

(fn `UserConstructionScript`)