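; Testing grounds game mode that lays a chain of BP_Tile actors, starting with two spawns at BeginPlay.
; SpawnTile places each tile at the previous tile's arrow attach transform and hands it the NavPool.
; ManageTilePool keeps a short rolling window of tiles, destroying the oldest once the limit is exceeded.
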(event `self.ReceiveBeginPlay`
  (set `self.Transform` (`KismetMathLibrary.MakeTransform` (0.0 0.0 0.0)))
  (for _ (range 2)
    (`self.SpawnTile`)))

(fn `ManageTilePool`
  (params (NewItem :type "Actor Object Reference (by ref)"))
  (bind _currenttiles (`self.CurrentTiles`))
  (bind _currenttiles_2 (`self.CurrentTiles`))
  (bind _output (`|GetArrayItem` _currenttiles_2))
  (`KismetArrayLibrary.Array_Add` _currenttiles NewItem)
  (if (> (`KismetArrayLibrary.Array_Length` _currenttiles) 3)
    (bind _output_get (set `self.ToDestroy` _output))
    (`KismetArrayLibrary.Array_RemoveItem` _currenttiles_2 _output)
    (`self.K2_DestroyActor` _output_get)))

(fn `SpawnTile`
  (bind _spawnedtile (`self.SpawnedTile`))
  (bind _returnvalue (`|SpawnActorFromClass` "/Game/Dynamic/Tiles/Behaviour/BP_Tile.BP_Tile_C" (`self.Transform`) "Undefined" "OverrideRootScale" null null))
  (bind _output_get (set `self.SpawnedTile` _returnvalue))
  (set `self.Transform` (`/Game/Dynamic/Tiles/Behaviour/BP_Tile.GetArrowAttachLocation` _output_get))
  (`Tile.SetPool` _spawnedtile (`self.NavPool`))
  (`self.ManageTilePool` _spawnedtile))

(fn `UserConstructionScript`)