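; BP_Tile is a level tile that scatters random props and gates the player behind a curtain barrier.
; BeginPlay locks the curtain and calls PlaceActors for containers, boxes, canisters, rocks and sack piles.
; Player overlap with LockingVolume turns the curtain green and passable, and leaving the curtain relocks it red and blocking.
; Leaving LockingVolume asks BP_TestingGroundsGM to spawn another tile, and the Arrow exposes an attach transform.
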(event `self.ReceiveBeginPlay`
  (`self.Lock`)
  (`self.PlaceActors` "/Game/Dynamic/Terrain/Props/BP_Container.BP_Container_C" 1 3)
  (`self.PlaceActors` "/Game/Dynamic/Terrain/Props/BP_Box2.BP_Box2_C" 2 6)
  (`self.PlaceActors` "/Game/Dynamic/Terrain/Props/BP_Canister1.BP_Canister1_C" 2 8)
  (`self.PlaceActors` "/Game/Dynamic/Terrain/Props/BP_Rock01.BP_Rock01_C" 2 8)
  (`self.PlaceActors` "/Game/Dynamic/Terrain/Props/BP_Rock17.BP_Rock17_C" 2 8)
  (`self.PlaceActors` "/Game/Dynamic/Terrain/Props/BP_SackPile.BP_SackPile_C" 1 3))

(event `self.Curtain.OnComponentEndOverlap`
  (params (OverlappedComponent :type "PrimitiveComponent Object Reference") (OtherActor :type "Actor Object Reference") (OtherComp :type "PrimitiveComponent Object Reference") (OtherBodyIndex :type Integer))
  (`self.IsPlayer` OtherActor
    (:`True`
      (`self.Lock`))))

(event `self.LockingVolume.OnComponentBeginOverlap`
  (params (OverlappedComponent :type "PrimitiveComponent Object Reference") (OtherActor :type "Actor Object Reference") (OtherComp :type "PrimitiveComponent Object Reference") (OtherBodyIndex :type Integer) (bFromSweep :type Boolean) (SweepResult :type "HitResult Structure (by ref)"))
  (`self.IsPlayer` OtherActor
    (:`True`
      (`self.Unlock`))))

(event `self.LockingVolume.OnComponentEndOverlap`
  (params (OverlappedComponent :type "PrimitiveComponent Object Reference") (OtherActor :type "Actor Object Reference") (OtherComp :type "PrimitiveComponent Object Reference") (OtherBodyIndex :type Integer))
  (`self.IsPlayer` OtherActor
    (:`True`
      (bind _asbp_testing_grounds_gm (cast `/Game/Dynamic/GM/BP_TestingGroundsGM` (`GameplayStatics.GetGameMode`)))
      (`/Game/Dynamic/GM/BP_TestingGroundsGM.SpawnTile` _asbp_testing_grounds_gm))))

(fn `GetArrowAttachLocation`
  (returns (Transform :type "Transform Structure"))
  (return (`SceneComponent.K2_GetComponentToWorld` (`self.Arrow`))))

(fn `Lock`
  (bind _curtain (`self.Curtain`))
  (`PrimitiveComponent.SetCollisionResponseToAllChannels` _curtain "ECR_Block")
  (`PrimitiveComponent.SetMaterial` _curtain 0 "/Game/Static/Geometry/Meshes/MI_Barrier_Red.MI_Barrier_Red"))

(fn `Unlock`
  (bind _curtain (`self.Curtain`))
  (`PrimitiveComponent.SetCollisionResponseToAllChannels` _curtain "ECR_Overlap")
  (`PrimitiveComponent.SetMaterial` _curtain 0 "/Game/Static/Geometry/Meshes/MI_Barrier_Green.MI_Barrier_Green"))

(fn `UserConstructionScript`)